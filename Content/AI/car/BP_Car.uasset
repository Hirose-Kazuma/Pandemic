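; AI traffic car that drives itself along a 2D heading each tick while riding is enabled.
; Overlapping a BP_Intersection picks a turn, and left or right turns step the heading to 90 degrees at a speed set by the intersection's X scale.
; StopRed and GoBlue halt and resume it, and a second box makes it queue behind red-stopped cars.
; Timeline-based gradual braking and acceleration are present but unconnected.
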(event OnComponentBeginOverlap(Box)
  (params (OverlappedComponent :type Primitive%20Component%20Object%20Reference) (OtherActor :type Actor%20Object%20Reference) (OtherComp :type Primitive%20Component%20Object%20Reference) (OtherBodyIndex :type Integer) (bFromSweep :type Boolean) (SweepResult :type Hit%20Result%20Structure%20%28by%20ref%29))
  (bind _asbp_intersection (Utilities|Casting|CastToBP_Intersection OtherActor))
  (bind _turntype (Default|TurnSelect _asbp_intersection self))
  (CallFunction|InIntersection _turntype (.x (Transformation|GetActorScale3D _asbp_intersection))))

(event OnComponentEndOverlap(Box)
  (params (OverlappedComponent :type Primitive%20Component%20Object%20Reference) (OtherActor :type Actor%20Object%20Reference) (OtherComp :type Primitive%20Component%20Object%20Reference) (OtherBodyIndex :type Integer))
  (Utilities|Casting|CastToBP_Intersection OtherActor))

(event OnComponentEndOverlap(Box1)
  (params (OverlappedComponent :type Primitive%20Component%20Object%20Reference) (OtherActor :type Actor%20Object%20Reference) (OtherComp :type Primitive%20Component%20Object%20Reference) (OtherBodyIndex :type Integer))
  (Utilities|Casting|CastToBP_Car OtherActor)
  (Variables|Default|SetIsRedStop false)
  (Variables|Default|Setspeed (Variables|Default|GetResetSpeed)))

(event OnComponentBeginOverlap(Box1)
  (params (OverlappedComponent :type Primitive%20Component%20Object%20Reference) (OtherActor :type Actor%20Object%20Reference) (OtherComp :type Primitive%20Component%20Object%20Reference) (OtherBodyIndex :type Integer) (bFromSweep :type Boolean) (SweepResult :type Hit%20Result%20Structure%20%28by%20ref%29))
  (bind _asbp_car (Utilities|Casting|CastToBP_Car OtherActor))
  (if (Variables|BP_Car_C|GetIsRedStop _asbp_car)
    (Variables|Default|SetIsRedStop true)
    (Variables|Default|Setspeed 0.0)))

(event EventBeginPlay
  (bind _basespeed (Variables|Default|GetbaseSpeed))
  (Variables|Default|Setpos (Transformation|GetActorLocation self))
  (Variables|Default|Setspeed _basespeed)
  (Variables|Default|SetResetSpeed _basespeed))

(event Collision|EventActorBeginOverlap
  (params (OtherActor :type Actor%20Object%20Reference)))

(event EventTick
  (params (DeltaSeconds :type Float%20%28single-precision%29))
  (bind _returnvalue (Math|Vector2D|MakeVector2D 1.0 0.0))
  (bind _basespeed (Variables|Default|GetbaseSpeed))
  (if (and (Variables|Default|GetisRide) (!= (Variables|Default|Getspeed) 0.0))
    (bind _output_get (Variables|Default|Setpos (+ (Variables|Default|Getpos) (* (Math|Vector|MakeVector (.x (Variables|Default|GetmoveVec)) (.y (Variables|Default|GetmoveVec)) 0.0) (Variables|Default|Getspeed)))))
    (Transformation|SetActorLocation _output_get false false)
    (if (Variables|Default|GetisIntersection)
      (Variables|Default|SetmoveVec (CallFunction|FAddition (Variables|Default|GetmoveVec) (Variables|Default|Getrot)))
      (if (>= (CallFunction|FDot (Variables|Default|GetmoveVec) (Variables|Default|GetbaseVec)) 9e+01)
        (Variables|Default|SetmoveVec (CallFunction|FAddition (Variables|Default|GetbaseVec) (Variables|Default|GetbaseTurn)))
        (Variables|Default|SetisIntersection false)
        (Variables|Default|Setspeed _basespeed)
        (Variables|Default|SetResetSpeed _basespeed))
      (Transformation|SetActorRotation (Math|Rotator|MakeRotator 0.0 0.0 (* (CallFunction|FDot (Variables|Default|GetmoveVec) _returnvalue) (CallFunction|FCross (Variables|Default|GetmoveVec) _returnvalue)))))))

(fn ConstructionScript)

(fn SetRide
  (params (flg :type Boolean))
  (Variables|Default|SetisRide flg))

(fn InIntersection
  (params (TurnType :type E_TurnType%20Enum :default "NewEnumerator2") (HandolRot :type Float%20%28single-precision%29))
  (bind _returnvalue (* HandolRot 0.5))
  (switch Utilities|FlowControl|Switch|SwitchonE_TurnType TurnType
    (:NewEnumerator2
      (Variables|Default|SetbaseVec (Variables|Default|GetmoveVec))
      (Variables|Default|SetisIntersection true)
      (Variables|Default|SetResetSpeed _returnvalue)
      (Variables|Default|Setspeed _returnvalue)
      (Variables|Default|SetbaseTurn -9e+01)
      (Variables|Default|Setrot -1.0))
    (:NewEnumerator0
      (Variables|Default|SetbaseVec (Variables|Default|GetmoveVec))
      (Variables|Default|SetisIntersection true)
      (Variables|Default|SetResetSpeed HandolRot)
      (Variables|Default|Setspeed HandolRot)
      (Variables|Default|SetbaseTurn 9e+01)
      (Variables|Default|Setrot 1.0))))

(fn StopRed
  (Variables|Default|SetIsRedStop true)
  (Variables|Default|Setspeed 0.0))

(fn GoBlue
  (Variables|Default|SetIsRedStop false)
  (Variables|Default|Setspeed (Variables|Default|GetResetSpeed)))