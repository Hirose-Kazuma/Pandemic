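; Road intersection actor for AI cars that chooses a random turn type for a given car.
; On BeginPlay it stores its North, East, South and West direction flags in an array.
; TurnSelect classifies the car's side by comparing a 2D cross-times-dot product against degree-style thresholds.
; A LoopBreak-controlled loop rerolls the turn offset, wrapping around the array, until it hits an enabled direction, then returns it as E_TurnType.
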(event EventBeginPlay
  (bind _direction (Variables|Default|GetDirection))
  (Variables|Default|SetDirectionFlg (Utilities|Array|MakeArray (.north _direction) (.east _direction) (.south _direction) (.west _direction))))

(event Collision|EventActorBeginOverlap
  (params (OtherActor :type Actor%20Object%20Reference)))

(event EventTick
  (params (DeltaSeconds :type Float%20%28single-precision%29)))

(fn ConstructionScript)

(fn TurnSelect
  (params (actor :type Actor%20Object%20Reference))
  (bind _returnvalue (Transformation|GetActorLocation))
  (bind _returnvalue_2 (Transformation|GetActorLocation actor))
  (bind _returnvalue_3 (Math|Vector2D|MakeVector2D 1.0 0.0))
  (bind _directionflg (Variables|Default|GetDirectionFlg))
  (bind _returnvalue_4 (Utilities|Array|Length _directionflg))
  (bind _returnvalue_5 (Math|Conversions|ToVector2D(Vector) _returnvalue))
  (bind _returnvalue_6 (Math|Conversions|ToVector2D(Vector) _returnvalue_2))
  (bind _returnvalue_7 (- _returnvalue_6 _returnvalue_5))
  (bind _returnvalue_8 (Math|Vector2D|Normalize2D _returnvalue_7))
  (bind _sign (CallFunction|FCross _returnvalue_3 _returnvalue_8))
  (bind _degree (CallFunction|FDot _returnvalue_3 _returnvalue_8))
  (bind _returnvalue_9 (* _sign _degree))
  (if (<= _returnvalue_9 -135.0)
    (LocalVariables|SetActorDirection "NewEnumerator2" :!label _label)
    (elif (<= _returnvalue_9 -45.0)
      (LocalVariables|SetActorDirection "NewEnumerator1")
      (elif (<= _returnvalue_9 45.0)
        (LocalVariables|SetActorDirection "NewEnumerator0")
        (elif (<= _returnvalue_9 135.0)
          (LocalVariables|SetActorDirection "NewEnumerator3")
          (else
            (goto _label))))))
  (while (LocalVariables|GetloopBreak)
    (LocalVariables|Set_turnType (Math|Random|RandomIntegerinRange 1 3))
    (if (>= (+ (Math|Conversions|ToInteger(Byte) (LocalVariables|GetActorDirection)) (LocalVariables|Get_turnType)) _returnvalue_4)
      (LocalVariables|SetloopBreak (not (Utilities|Array|Get(acopy) (Variables|Default|GetDirectionFlg) (- (+ (Math|Conversions|ToInteger(Byte) (LocalVariables|GetActorDirection)) (LocalVariables|Get_turnType)) _returnvalue_4))))
      (else
        (LocalVariables|SetloopBreak (not (Utilities|Array|Get(acopy) (Variables|Default|GetDirectionFlg) (+ (Math|Conversions|ToInteger(Byte) (LocalVariables|GetActorDirection)) (LocalVariables|Get_turnType))))))))
  (return (Utilities|Enum|ByteToEnumE_TurnType (Math|Conversions|ToByte(Integer) (- (LocalVariables|Get_turnType) 1)))))