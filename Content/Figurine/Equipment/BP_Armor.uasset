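; BP_Armor is an armor pickup that equips itself onto a BP_TpOwner when that actor overlaps its sphere.
; The overlap passes the owner to EquipItem, which snaps the root component to the world transform of the EquipSocket socket on the owner's mesh.
; It then attaches the root to that socket's parent bone, keeping world location, rotation and scale.
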(event OnComponentBeginOverlap(Sphere)
  (params (OverlappedComponent :type Primitive%20Component%20Object%20Reference) (OtherActor :type Actor%20Object%20Reference) (OtherComp :type Primitive%20Component%20Object%20Reference) (OtherBodyIndex :type Integer) (bFromSweep :type Boolean) (SweepResult :type Hit%20Result%20Structure%20%28by%20ref%29))
  (bind _asbp_tp_owner (Utilities|Casting|CastToBP_TpOwner OtherActor))
  (CallFunction|EquipItem _asbp_tp_owner))

(fn ConstructionScript)

(fn EquipItem
  (params (InputPin :type BP%20Tp%20Owner%20Object%20Reference))
  (bind _mesh (Variables|/Script/Engine.Character|GetMesh InputPin))
  (Transformation|SetWorldTransform (Variables|Default|GetDefaultSceneRoot) (Transformation|GetSocketTransform _mesh (Variables|Default|GetEquipSocket) "RTS_World") false false)
  (Transformation|AttachComponentToComponent (Variables|Default|GetDefaultSceneRoot) _mesh (Class|SkinnedMeshComponent|GetSocketBoneName _mesh (Variables|Default|GetEquipSocket)) "KeepWorld" "KeepWorld" "KeepWorld" true))