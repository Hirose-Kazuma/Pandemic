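; BP_Door is a door actor that, as written, only prints debug information when the player leaves its Box trigger and does not open or move.
; On end overlap it casts to BP_Player, filters for components whose display name contains "cylinder", and prints the vector from player to door.
; Unconnected leftover nodes would toggle a test flag and print a forward direction, but never run.
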(event OnComponentEndOverlap(Box)
  (params (OverlappedComponent :type Primitive%20Component%20Object%20Reference) (OtherActor :type Actor%20Object%20Reference) (OtherComp :type Primitive%20Component%20Object%20Reference) (OtherBodyIndex :type Integer))
  (bind _asbp_player (Utilities|Casting|CastToBP_Player OtherActor))
  (if (Utilities|String|Contains (Utilities|GetDisplayName OtherComp) "cylinder")
    (Development|PrintString (Utilities|String|ToString(Vector) (- (Transformation|GetActorLocation self) (Transformation|GetActorLocation _asbp_player))))))

(event EventBeginPlay)

(event Collision|EventActorBeginOverlap
  (params (OtherActor :type Actor%20Object%20Reference)))

(event EventTick
  (params (DeltaSeconds :type Float%20%28single-precision%29)))

(fn ConstructionScript)