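; Character for citizens and zombies in an infection game, with dash, jump, bite and a launch that detaches the upper body.
; Infecting a citizen passes player control and stats to the victim, leaving the old body to AICon_Enemy; AI infections create AI zombies.
; Player transfers fill an evolution gauge that upgrades GameInstance zombie stats by dominant action counts.
; Zombies ragdoll when their life timer expires; the player jumps to the nearest infected.
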(event OnComponentBeginOverlap(CoughCollision)
  (params (OverlappedComponent :type Primitive%20Component%20Object%20Reference) (OtherActor :type Actor%20Object%20Reference) (OtherComp :type Primitive%20Component%20Object%20Reference) (OtherBodyIndex :type Integer) (bFromSweep :type Boolean) (SweepResult :type Hit%20Result%20Structure%20%28by%20ref%29))
  (bind _walkspeed (Variables|Default|GetWalkSpeed))
  (bind _walkspeed_2 (Variables|Default|GetWalkSpeed))
  ;[1 1 1] 当たり判定
  (bind _asbp_tp_owner (Utilities|Casting|CastToBP_TpOwner OtherActor))
  (if (Math|Boolean|ANDBoolean (!= _asbp_tp_owner self) (Variables|Default|GetIsInfection) (not (Variables|Default|GetIsDead)))
    (Utilities|Array|Add (Variables|Default|GetBiteList) _asbp_tp_owner)
    (if (> (Utilities|Array|Length (Variables|Default|GetBiteList)) 1)
      (Variables|Default|SetTouchTp (Utilities|Array|Get(acopy) (Variables|Default|GetBiteList)))
      (else
        (Variables|Default|SetTouchTp _asbp_tp_owner)))
    (if (not (Variables|BP_TpOwner_C|GetIsInfection (Variables|Default|GetTouchTp)))
      (Variables|BP_TpOwner_C|SetIsInfection (Variables|Default|GetTouchTp) true)
      (Rendering|Material|SetMaterial (Variables|/Script/Engine.Character|GetMesh (Variables|Default|GetTouchTp)) 0 "/Game/Character/Material/M_Red.M_Red")
      (Default|SetCitizen (Variables|Default|GetMyGameInstance) (Utilities|Struct|MakeS_CitizenStatus 0.0 -1.0 1.0 0.0))
      ;[1 1 1] チェンジ
      (Utilities|PlayerChange (Variables|Default|GetTouchTp))
      ;[1 1 1] ダッシュ継続
      (if (> (Variables|/Script/Engine.CharacterMovementComponent|GetMaxWalkSpeed (Variables|Character|GetCharacterMovement)) (* (.walkspeed _walkspeed_2) (.zombiespeedratio _walkspeed_2)))
        (Variables|/Script/Engine.CharacterMovementComponent|SetMaxWalkSpeed (Variables|/Script/Engine.Character|GetCharacterMovement (Variables|Default|GetTouchTp)) (* (.runspeed _walkspeed) (.zombiespeedratio _walkspeed)))))))

(event Custom|LivingDead
  (params (ターゲット :type BP%20Tp%20Owner%20Object%20Reference))
  ;[1 1 1] 生き返り
  (Utilities|PlayerChange ターゲット))

(event Custom|CameraResetStart
  ;[1 1 1] カメラリセット
  (Timeline|CameraReset PlayFromStart
    (:Update
      (CallFunction|CameraResetTick))))

(event Custom|CameraResetEnd
  ;[1 1 1] カメラリセット
  (Timeline|CameraReset Stop
    (:Update
      (CallFunction|CameraResetTick))))

(event Custom|AIBite
  ;[1 1 1] 噛みつき
  (if (Utilities|Enum|Equal(Enum) (Variables|Default|GetMyStatus) "NewEnumerator0")
    (Variables|Default|SetMyStatus "NewEnumerator6")
    (Variables|/Script/Engine.CharacterMovementComponent|SetMaxWalkSpeed (Variables|Character|GetCharacterMovement) 2e+03)))

(event Custom|AIDash
  (bind _walkspeed (Variables|Default|GetWalkSpeed))
  (bind _charactermovement (Variables|Character|GetCharacterMovement))
  ;[1 1 1] ダッシュ
  (if (Variables|Default|GetIsInfection)
    (Variables|/Script/Engine.CharacterMovementComponent|SetMaxWalkSpeed _charactermovement (* (.runspeed _walkspeed) (.zombiespeedratio _walkspeed)))
    (else
      (Variables|/Script/Engine.CharacterMovementComponent|SetMaxWalkSpeed _charactermovement (.runspeed (Variables|Default|GetWalkSpeed))))))

(event EventTick
  (params (DeltaSeconds :type Float%20%28single-precision%29))
  ;[0.4219 0.5401 1] Tick
  (Utilities|FlowControl|Sequence
    (:then_0
      (CallFunction|TouchCollision)
      (CallFunction|BodyExpansion)
      (CallFunction|LifeLimitTimer DeltaSeconds))))

(event EventBeginPlay
  ;[1 0.4583 0.4623] BeginPlay
  (Variables|Default|SetLifeLimit (Variables|Default|GetDefaultLifeLimit))
  (Variables|Default|SetMyGameInstance (.AsBP%20My%20Game%20Instance (Utilities|Casting|CastToBP_MyGameInstance (Game|GetGameInstance)))))

(event Input|ActionEvents|InputActionBite
  (params (Key :type Key%20Structure))
  ;[1 1 1] 噛みつき
  (:Pressed
    (if (Utilities|Enum|Equal(Enum) (Variables|Default|GetMyStatus) "NewEnumerator0")
      (Variables|Default|SetMyStatus "NewEnumerator6")
      (Variables|/Script/Engine.CharacterMovementComponent|SetMaxWalkSpeed (Variables|Character|GetCharacterMovement) 2e+03))))

(event Input|ActionEvents|InputActionLastAttack
  (params (Key :type Key%20Structure))
  (bind _returnvalue (Transformation|GetActorTransform))
  (bind _mesh (Variables|Character|GetMesh))
  ;[1 1 1] 上半身ロケット
  (:Pressed
    (if (Variables|Default|GetIsBodyShot)
      (if (== (Math|Vector|VectorLength (Variables|/Script/Engine.MovementComponent|GetVelocity (Variables|Character|GetCharacterMovement))) 0.0)
        (Character|LaunchCharacter (* (+ (Transformation|GetActorForwardVector) (Math|Vector|MakeVector 0.0 0.0 0.2)) (/ (Variables|Default|GetLastAttackForce) 3.0)) false false)
        (Utilities|Array|Clear (Variables|Default|GetBiteList)))
      (else
        (Variables|Default|SetMyStatus "NewEnumerator8"))))
  (:Released
    (if (not (Variables|Default|GetIsBodyShot))
      (Variables|Default|SetIsBodyShot true)
      (Variables|Default|SetMyStatus "NewEnumerator7")
      (Character|LaunchCharacter (* (+ (Transformation|GetActorForwardVector) (Math|Vector|MakeVector 0.0 0.0 0.174)) (Variables|Default|GetLastAttackForce)) false false)
      (Game|SpawnActorfromClass "/Game/Character/BP_UnderBody.BP_UnderBody_C" (Math|Transform|MakeTransform (+ (* (Transformation|GetActorForwardVector) -2e+02) (.location _returnvalue)) (.rotation _returnvalue) (.scale _returnvalue)) "Undefined" 0 0)
      (Components|SkinnedMesh|HideBonebyName _mesh "thigh_r" "PBO_Term")
      (Components|SkinnedMesh|HideBonebyName _mesh "thigh_l" "PBO_Term")
      (Components|Capsule|SetCapsuleHalfHeight (Variables|Collision|GetCapsuleComponent) 42.0 true)
      (CallFunction|StatusMonitoring (Utilities|Struct|MakeS_PlayerBonus 0.0 0.0 0.0 3e+01))
      (Default|SoundManager (Variables|Default|GetMyGameInstance) "NewEnumerator1"))))

(event Input|ActionEvents|InputActionDush
  (params (Key :type Key%20Structure))
  (bind _walkspeed (Variables|Default|GetWalkSpeed))
  (bind _walkspeed_2 (Variables|Default|GetWalkSpeed))
  (bind _charactermovement (Variables|Character|GetCharacterMovement))
  (bind _charactermovement_2 (Variables|Character|GetCharacterMovement))
  ;[1 1 1] ダッシュ
  (:Pressed
    (if (Variables|Default|GetIsInfection)
      (Variables|/Script/Engine.CharacterMovementComponent|SetMaxWalkSpeed _charactermovement (* (.runspeed _walkspeed_2) (.zombiespeedratio _walkspeed_2)))
      (else
        (Variables|/Script/Engine.CharacterMovementComponent|SetMaxWalkSpeed _charactermovement (.runspeed (Variables|Default|GetWalkSpeed))))))
  (:Released
    (if (Variables|Default|GetIsInfection)
      (Variables|/Script/Engine.CharacterMovementComponent|SetMaxWalkSpeed _charactermovement_2 (* (.walkspeed _walkspeed) (.zombiespeedratio _walkspeed)))
      (else
        (Variables|/Script/Engine.CharacterMovementComponent|SetMaxWalkSpeed _charactermovement_2 (.walkspeed (Variables|Default|GetWalkSpeed)))))))

(event Input|ActionEvents|InputActionCameraReset
  (params (Key :type Key%20Structure))
  ;[1 1 1] カメラリセット
  (:Pressed
    (Variables|Default|SetCameraResetFlag true)
    (Variables|Default|SetCameraResetRotation (Transformation|GetWorldRotation (Variables|Collision|GetCapsuleComponent)))
    (CallFunction|CameraResetStart)))

(event Input|ActionEvents|InputActionSpecial
  (params (Key :type Key%20Structure))
  ;[1 1 1] TEST
)

(event Input|ActionEvents|InputActionJump
  (params (Key :type Key%20Structure))
  ;[1 1 1] ジャンプ
  (:Pressed
    (if (and (Utilities|Enum|Equal(Enum) (Variables|Default|GetMyStatus) "NewEnumerator0") (not (Variables|Default|GetIsBodyShot)))
      (Character|Jump)
      (Variables|Default|SetMyStatus "NewEnumerator2")
      (CallFunction|StatusMonitoring (Utilities|Struct|MakeS_PlayerBonus 0.0 0.0 1e+01 0.0))))
  (:Released
    (Character|StopJumping)))

(event Input|AxisEvents|InputAxisTurnRate
  (params (AxisValue :type Float%20%28single-precision%29))
  (bind _springarm (Variables|Default|GetSpringArm))
  (bind _returnvalue (Transformation|GetWorldRotation _springarm))
  ;[1 1 1] ゲームパッドカメラ
  (if (not (Variables|Default|GetCameraResetFlag))
    (Transformation|SetWorldRotation (Variables|Default|GetSpringArm) (Math|Rotator|MakeRotator 0.0 (.pitch _returnvalue) (+ AxisValue (.yaw _returnvalue))) false false)))

(event Input|AxisEvents|InputAxisLookUpRate
  (params (AxisValue :type Float%20%28single-precision%29))
  (bind _springarm (Variables|Default|GetSpringArm))
  (bind _returnvalue (Transformation|GetWorldRotation _springarm))
  (bind _returnvalue_2 (- (.pitch _returnvalue) AxisValue))
  ;[1 1 1] ゲームパッドカメラ
  (if (and (<= (Math|Float|Absolute(Float) _returnvalue_2) 4e+01) (not (Variables|Default|GetCameraResetFlag)))
    (Transformation|SetWorldRotation (Variables|Default|GetSpringArm) (Math|Rotator|MakeRotator 0.0 _returnvalue_2 (.yaw _returnvalue)) false false)))

(event Input|AxisEvents|InputAxisMoveForward
  (params (AxisValue :type Float%20%28single-precision%29))
  ;[1 1 1] 移動
  (if (Utilities|Enum|Equal(Enum) (Variables|Default|GetMyStatus) "NewEnumerator0")
    (Pawn|Input|AddMovementInput (select (Variables|Default|GetIsBodyShot) "0, 0, 0" (Math|Vector|GetForwardVector (Variables|Default|GetCamera))) AxisValue false)
    (Variables|Default|SetStickDown (!= (+ AxisValue (stale Input|AxisEvents|InputAxisMoveRight AxisValue)) 0.0))))

(event Input|AxisEvents|InputAxisMoveRight
  (params (AxisValue :type Float%20%28single-precision%29))
  ;[1 1 1] 移動
  (if (Utilities|Enum|Equal(Enum) (Variables|Default|GetMyStatus) "NewEnumerator0")
    (Pawn|Input|AddMovementInput (select (Variables|Default|GetIsBodyShot) "0, 0, 0" (Math|Vector|GetRightVector (Variables|Default|GetCamera))) AxisValue false)
    (Variables|Default|SetStickDown (!= (+ (stale Input|AxisEvents|InputAxisMoveForward AxisValue) AxisValue) 0.0))))

(event Input|KeyboardEvents|Q
  (params (Key :type Key%20Structure))
  ;[1 1 1] TEST
)

(fn ConstructionScript)

(fn LifeLimitTimer
  (params (LifeLimit :type Float%20%28single-precision%29))
  (if (Variables|Default|GetIsInfection)
    (bind _output_get (Variables|Default|SetLifeLimit (- (Variables|Default|GetLifeLimit) LifeLimit)))
    (if (<= _output_get 0.0)
      (Collision|SetCollisionEnabled (Variables|Collision|GetCapsuleComponent) "NoCollision")
      (Class|SkeletalMeshComponent|SetAllBodiesSimulatePhysics (Variables|Character|GetMesh) true)
      (Variables|Default|SetIsInfection false)
      (Variables|Default|SetIsDead true)
      (Pawn|Components|CharacterMovement|DisableMovement (Variables|Character|GetCharacterMovement))
      (bind _returnvalue (Effects|SpawnEmitteratLocation "/Game/Effect/Particle/P_Death.P_Death" (- (Transformation|GetSocketLocation (Variables|Character|GetMesh) "head") "0,0.000000,30.000000")))
      (Transformation|AttachComponentToComponent _returnvalue (Variables|Character|GetMesh) "Bip-Mouth1" "KeepWorld" "KeepWorld" "KeepWorld" true)
      (Components|SkinnedMesh|HideBonebyName (Variables|Character|GetMesh) "Bip-Mouth1" "PBO_Term")
      (Default|SetCitizen (Variables|Default|GetMyGameInstance) (Utilities|Struct|MakeS_CitizenStatus 0.0 0.0 -1.0 1.0))
      (if (Variables|Default|GetIsOperationPlayer)
        (bind _output_get_2 (CallFunction|SerchNearTarget))
        (if (Utilities|IsValid _output_get_2)
          (CallFunction|LivingDead _output_get_2)
          (else
            (Development|PrintString "GAME OVER")))))))

(fn TouchCollision
  (bind _coughcollision (Variables|Default|GetCoughCollision))
  (if (or (and (Variables|Default|GetIsInfection) (Utilities|Enum|Equal(Enum) (Variables|Default|GetMyStatus) "NewEnumerator6")) (Variables|Default|GetIsBodyShot))
    (Utilities|FlowControl|DoOnce false :!label _label
      (:Completed
        (Collision|SetCollisionEnabled _coughcollision "QueryAndPhysics")
        (goto _label_2 Reset)))
    (else
      (Utilities|FlowControl|DoOnce false :!label _label_2
        (:Completed
          (Collision|SetCollisionEnabled _coughcollision "NoCollision")
          (goto _label Reset))))))

(fn BodyExpansion
  (if (Variables|Default|GetIsInfection)
    (Variables|Default|SetExpansionScale (+ (Variables|Default|GetExpansionScale) 0.01))))

(fn CameraResetTick
  (bind _springarm (Variables|Default|GetSpringArm))
  (bind _relativerotation (Variables|/Script/Engine.SceneComponent|GetRelativeRotation _springarm))
  (if (or (>= (Math|Float|Absolute(Float) (.pitch _relativerotation)) 0.3) (>= (Math|Float|Absolute(Float) (- (Math|Float|Absolute(Float) (.yaw _relativerotation)) (Math|Float|Absolute(Float) (.yaw (Transformation|GetWorldRotation (Variables|Collision|GetCapsuleComponent)))))) 0.3))
    (Transformation|SetRelativeRotation (Variables|Default|GetSpringArm) (Math|Interpolation|RInterpTo (Variables|/Script/Engine.SceneComponent|GetRelativeRotation (Variables|Default|GetSpringArm)) (Variables|Default|GetCameraResetRotation) (Utilities|Time|GetWorldDeltaSeconds) 15.0) false false)
    (else
      (Variables|Default|SetCameraResetFlag false)
      (CallFunction|CameraResetEnd))))

(fn StatusMonitoring
  (params (BonusCount :type S%20Player%20Bonus%20Structure))
  (bind _output_get (Variables|Default|SetPlayerBonus (Utilities|Struct|MakeS_PlayerBonus (+ (.speedcount BonusCount) (.speedcount (Variables|Default|GetPlayerBonus))) (+ (.lifecount BonusCount) (.lifecount (Variables|Default|GetPlayerBonus))) (+ (.jampcount BonusCount) (.jampcount (Variables|Default|GetPlayerBonus))) (+ (.lastattackcount BonusCount) (.lastattackcount (Variables|Default|GetPlayerBonus))))))
  (return _output_get))

(fn LevelUp
  (Variables|Default|SetEvolutionGauge 0.0)
  (Default|SoundManager (Variables|Default|GetMyGameInstance) "NewEnumerator0")
  (bind (_array_element _array_index) (Utilities|Array|ForEachLoopwithBreak (Utilities|Array|MakeArray (.speedcount (Variables|Default|GetPlayerBonus)) (.lifecount (Variables|Default|GetPlayerBonus)) (.jampcount (Variables|Default|GetPlayerBonus)) (.lastattackcount (Variables|Default|GetPlayerBonus))) :!label _label)
    (:LoopBody
      (if (== _array_element (Math|Float|Max(Float) (.speedcount (Variables|Default|GetPlayerBonus)) (.lifecount (Variables|Default|GetPlayerBonus)) (.jampcount (Variables|Default|GetPlayerBonus)) (.lastattackcount (Variables|Default|GetPlayerBonus))))
        (switch int _array_index
          (:0
            _)
          (:1
            (Variables|/Game/GameInstance/BP_MyGameInstance.BP_MyGameInstance_C|SetZombieStatus (Variables|Default|GetMyGameInstance) (Utilities|Struct|MakeS_ZombieStatus 0.0 (+ (Variables|Default|GetDefaultLifeLimit) 0.5) (Variables|/Script/Engine.CharacterMovementComponent|GetJumpZVelocity (Variables|Character|GetCharacterMovement)) (Variables|Default|GetLastAttackForce))))
          (:2
            (Variables|/Game/GameInstance/BP_MyGameInstance.BP_MyGameInstance_C|SetZombieStatus (Variables|Default|GetMyGameInstance) (Utilities|Struct|MakeS_ZombieStatus 0.0 (Variables|Default|GetDefaultLifeLimit) (+ (Variables|/Script/Engine.CharacterMovementComponent|GetJumpZVelocity (Variables|Character|GetCharacterMovement)) 5e+02) (Variables|Default|GetLastAttackForce))))
          (:3
            (Variables|/Game/GameInstance/BP_MyGameInstance.BP_MyGameInstance_C|SetZombieStatus (Variables|Default|GetMyGameInstance) (Utilities|Struct|MakeS_ZombieStatus 0.0 (Variables|Default|GetDefaultLifeLimit) (Variables|/Script/Engine.CharacterMovementComponent|GetJumpZVelocity (Variables|Character|GetCharacterMovement)) (+ (Variables|Default|GetLastAttackForce) 5e+02)))))
        (Variables|Default|SetPlayerBonus "")
        (goto _label Break)))))

(fn ZombeSet
  (params (PlayerBonus :type S%20Player%20Bonus%20Structure) (InputPin :type BP%20Tp%20Owner%20Object%20Reference))
  (bind _mygameinstance (Variables|Default|GetMyGameInstance))
  (bind _zombiestatus (Variables|/Game/GameInstance/BP_MyGameInstance.BP_MyGameInstance_C|GetZombieStatus _mygameinstance))
  (Variables|BP_TpOwner_C|SetPlayerBonus InputPin PlayerBonus)
  (Variables|BP_TpOwner_C|SetDefaultLifeLimit InputPin (.life _zombiestatus))
  (Variables|/Script/Engine.CharacterMovementComponent|SetJumpZVelocity (Variables|/Script/Engine.Character|GetCharacterMovement InputPin) (.jamp _zombiestatus))
  (Variables|BP_TpOwner_C|SetLastAttackForce InputPin (.rastattack _zombiestatus))
  (if (Variables|Default|GetIsOperationPlayer)
    (bind _output_get (Variables|BP_TpOwner_C|SetEvolutionGauge InputPin (+ (Variables|Default|GetEvolutionGauge) 1.0))) ; 進化ゲージプラス
    (if (>= _output_get (Variables|Default|GetEvolutionCount))
      (CallFunction|LevelUp InputPin)))
  (if (Variables|Default|GetIsDead)
    _
    (else
      (Variables|BP_TpOwner_C|SetLifeLimit InputPin (Variables|BP_TpOwner_C|GetDefaultLifeLimit InputPin))))
  (return))

(fn CameraSet
  (params (TouchTp_ref :type BP%20Tp%20Owner%20Object%20Reference))
  (Transformation|SetWorldRotation (Variables|BP_TpOwner_C|GetSpringArm TouchTp_ref) (Utilities|RotatioinPuls (Transformation|GetWorldRotation (Variables|/Script/Engine.Character|GetMesh TouchTp_ref)) (Transformation|GetWorldRotation (Variables|Default|GetSpringArm))) false false))

(fn SerchNearTarget
  (bind _outactors (Actor|GetAllActorsOfClass "BP_TpOwner_C"))
  (for _array_element _outactors
    (if (CallFunction|IsCanChange _array_element)
      (if (not (Utilities|IsValid (LocalVariables|Getnear)))
        (LocalVariables|Setnear _array_element)
        (LocalVariables|SetMinDistance (Transformation|GetDistanceTo _array_element self))
        (elif (< (Transformation|GetDistanceTo _array_element self) (LocalVariables|GetMinDistance))
          (LocalVariables|SetMinDistance (Transformation|GetDistanceTo _array_element self))
          (LocalVariables|Setnear _array_element)))))
  (return (LocalVariables|Getnear)))

(fn FallDown
  (params (fallDownFlg :type Boolean))
  (if fallDownFlg
    (Collision|SetCollisionEnabled (Variables|Collision|GetCapsuleComponent) "NoCollision")
    (Class|SkeletalMeshComponent|SetAllBodiesSimulatePhysics (Variables|Character|GetMesh) true)
    (else
      (Collision|SetCollisionEnabled (Variables|Collision|GetCapsuleComponent) "QueryAndPhysics")
      (Class|SkeletalMeshComponent|SetAllBodiesSimulatePhysics (Variables|Character|GetMesh) false))))

(fn IsCanChange
  (params (target :type BP%20Tp%20Owner%20Object%20Reference))
  (return (Math|Boolean|ANDBoolean (!= target self) (Variables|BP_TpOwner_C|GetIsInfection target) (not (Variables|BP_TpOwner_C|GetIsDead target)))))