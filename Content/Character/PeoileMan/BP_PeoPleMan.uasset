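; BP_PeoPleMan is a child character Blueprint that starts play as an infected, player-operated citizen.
; On BeginPlay it runs the parent logic, sets the player and infection flags, and shifts one citizen from uninfected to infected in the game instance.
; It also writes the game instance's ZombieStatus from its life limit, jump velocity and last attack force.
; Tick and the construction script only call the parent.
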(event EventBeginPlay
  (bind _mygameinstance (Variables|Default|GetMyGameInstance))
  (|CallParentFunction)
  (Variables|Default|SetIsOperationPlayer true)
  (Variables|Default|SetIsInfection true)
  (Default|SetCitizen _mygameinstance (Utilities|Struct|MakeS_CitizenStatus 0.0 -1.0 1.0 0.0))
  (Variables|/Game/GameInstance/BP_MyGameInstance.BP_MyGameInstance_C|SetZombieStatus _mygameinstance (Utilities|Struct|MakeS_ZombieStatus 0.0 (Variables|Default|GetDefaultLifeLimit) (Variables|/Script/Engine.CharacterMovementComponent|GetJumpZVelocity (Variables|Character|GetCharacterMovement)) (Variables|Default|GetLastAttackForce))))

(event Collision|EventActorBeginOverlap
  (params (OtherActor :type Actor%20Object%20Reference)))

(event EventTick
  (params (DeltaSeconds :type Float%20%28single-precision%29))
  (|CallParentFunction DeltaSeconds))

(fn ConstructionScript
  (|CallParentFunction))