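; Game instance that keeps a running tally of citizen status across the game: citizen, not-infected, infected and dead counts.
; SetCitizen treats its input struct as deltas, adding each non-zero field to the stored CitizenStatus, and GetCitizen returns that struct.
; A separate SoundManager function plays the LevelUp 2D sound.
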(fn SoundManager
  (Audio|PlaySound2D "/Game/Sounds/LevelUp.LevelUp"))

(fn SetCitizen
  (params (citizen :type S%20Citizen%20Status%20Structure))
  (if (!= (.citizen citizen) 0.0)
    (Variables|Default|SetCitizenStatus (Utilities|Struct|MakeS_CitizenStatus (+ (.citizen citizen) (.citizen (Variables|Default|GetCitizenStatus))) (.notinfection (Variables|Default|GetCitizenStatus)) (.infection (Variables|Default|GetCitizenStatus)) (.dead (Variables|Default|GetCitizenStatus)))))
  (if (!= (.notinfection citizen) 0.0)
    (Variables|Default|SetCitizenStatus (Utilities|Struct|MakeS_CitizenStatus (.citizen (Variables|Default|GetCitizenStatus)) (+ (.notinfection citizen) (.notinfection (Variables|Default|GetCitizenStatus))) (.infection (Variables|Default|GetCitizenStatus)) (.dead (Variables|Default|GetCitizenStatus)))))
  (if (!= (.infection citizen) 0.0)
    (Variables|Default|SetCitizenStatus (Utilities|Struct|MakeS_CitizenStatus (.citizen (Variables|Default|GetCitizenStatus)) (.notinfection (Variables|Default|GetCitizenStatus)) (+ (.infection citizen) (.infection (Variables|Default|GetCitizenStatus))) (.dead (Variables|Default|GetCitizenStatus)))))
  (if (!= (.dead citizen) 0.0)
    (Variables|Default|SetCitizenStatus (Utilities|Struct|MakeS_CitizenStatus (.citizen (Variables|Default|GetCitizenStatus)) (.notinfection (Variables|Default|GetCitizenStatus)) (.infection (Variables|Default|GetCitizenStatus)) (+ (.dead citizen) (.dead (Variables|Default|GetCitizenStatus)))))))

(fn GetCitizen
  (return (Variables|Default|GetCitizenStatus)))